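; BP_Key is a spinning key pickup linked to a door through DoorRef.
; The construction script applies a configurable mesh and pickup sound.
; Tick yaws the actor at a constant, frame-rate-independent speed.
; Its interaction event sets the door's DoorBlocked flag to true, plays the sound in 2D, then destroys the key after a short delay.
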(event EventBeginPlay)

(event Collision|EventActorBeginOverlap
  (params (OtherActor :type Actor%20Object%20Reference)))

(event EventIntereaction
  (params (Player%20location :type Vector :default "0, 0, 0"))
  (Variables|/Game/BluePrints/Door/BP_Door.BP_Door_C|SetDoor%20Blocked? (Variables|Ajustes|GetDoor%20Ref) true)
  (Audio|PlaySound2D (Variables|Default|GetSound%20key) 1.0 1.0 0.0 0 0)
  (Utilities|FlowControl|Delay 0.2)
  (Actor|DestroyActor))

(event EventTick
  (params (DeltaSeconds :type Float%20%28single-precision%29))
  (Transformation|AddActorLocalRotation (Math|Rotator|MakeRotator 0.0 0.0 (* DeltaSeconds 9e+01)) false false))

(fn ConstructionScript
  (Components|StaticMesh|SetStaticMesh (Variables|Default|GetKey) (Variables|Ajustes|GetMesh%20Key))
  (Variables|Default|SetSound%20key (Variables|Ajustes|GetNew%20Soun%20Key)))