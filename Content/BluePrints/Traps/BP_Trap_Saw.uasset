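; BP_Trap_Saw is a saw trap that damages actors it touches.
; On BeginPlay, two timelines animate the Saw component: LeftAndRight moves it along its local Y axis, and Spin rotates it around X.
; Overlapping the Saw applies fixed damage to the other actor and prints a debug message, with no filtering by actor type.
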(event OnComponentBeginOverlap(Saw)
  (params (OverlappedComponent :type Primitive%20Component%20Object%20Reference) (OtherActor :type Actor%20Object%20Reference) (OtherComp :type Primitive%20Component%20Object%20Reference) (OtherBodyIndex :type Integer) (bFromSweep :type Boolean) (SweepResult :type Hit%20Result%20Structure%20%28by%20ref%29))
  (Game|Damage|ApplyDamage OtherActor 1e+01 0 0)
  (Development|PrintString "hace daño"))

(event EventBeginPlay
  (Utilities|FlowControl|Sequence
    (:then_0
      (bind _move (Timeline|LeftAndRight Play)
        (:Update
          (Transformation|SetRelativeLocation (Variables|Default|GetSaw) (Math|Vector|Lerp(Vector) "0, 0, 0" "0.000000,330.000000,0.000000" _move) false false))))
    (:then_1
      (bind _newtrack_1 (Timeline|Spin Play)
        (:Update
          (Transformation|SetRelativeRotation (Variables|Default|GetSaw) (Math|Rotator|MakeRotator _newtrack_1 0.0 0.0) false false))))))

(fn ConstructionScript)