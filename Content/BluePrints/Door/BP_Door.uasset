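; BP_Door is an interactable door that swings open and closed on alternate interactions.
; A dot product between its forward vector and the direction to the player selects the swing direction.
; The Door_Rotation timeline plays or reverses through a FlipFlop, easing out the door's relative yaw.
; Despite its name, DoorBlocked must be true for movement; when false, only the blocked-door sound plays.
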(event EventIntereaction
  (params (Player%20location :type Vector :default "0, 0, 0"))
  (if (Variables|Ajustes|GetDoor%20Blocked?)
    (Audio|PlaySound2D "/Game/BluePrints/Door/Sounds/Puerta_cerrar.Puerta_cerrar" 1.0 1.0 0.0 0 0)
    (Utilities|FlowControl|FlipFlop
      (:A
        (Variables|Default|SetDoor%20Orientation (Math|Float|SelectFloat -1e+02 1e+02 (>= (Math|Vector|DotProduct (Math|Vector|GetUnitDirection(Vector) (Transformation|GetActorLocation) Player%20location) (Transformation|GetActorForwardVector)) 0.0)))
        (bind _alpha (Timeline|Door_Rotation Play)
          (:Update
            (Transformation|SetRelativeRotation (Variables|Default|GetDoor) (Math|Rotator|MakeRotator 0.0 0.0 (Math|Interpolation|Ease "EaseOut" _alpha 0.0 (Variables|Default|GetDoor%20Orientation) 2.0)) false false))))
      (:B
        (Timeline|Door_Rotation Reverse)))
    (else
      (Audio|PlaySound2D "/Game/BluePrints/Door/Sounds/blocked_door.blocked_door" 1.0 1.0 0.0 0 0))))

(fn ConstructionScript)