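; BP_Runes is a Blueprint with a rune mesh that temporarily relocates after its trigger box is overlapped.
; It caches the mesh's starting world location on BeginPlay.
; An overlap, ignored while IsActive is set, waits briefly, teleportlessly jumps the mesh without sweep, then restores it after a second delay.
; The target puts the starting Z minus an offset into X, zeroing Y and Z, rather than simply lowering it.
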(event OnComponentBeginOverlap(TriggerBox)
  (params (OverlappedComponent :type Primitive%20Component%20Object%20Reference) (OtherActor :type Actor%20Object%20Reference) (OtherComp :type Primitive%20Component%20Object%20Reference) (OtherBodyIndex :type Integer) (bFromSweep :type Boolean) (SweepResult :type Hit%20Result%20Structure%20%28by%20ref%29))
  (if (not (Variables|Default|GetIsActive))
    (Utilities|FlowControl|Delay 2.0)
    (bind _sweephitresult (Transformation|SetWorldLocation (Variables|Default|GetRuneMesh) (Math|Vector|MakeVector (- (.Z (Math|Vector|BreakVector (Variables|Default|GetInitialLocation))) 5e+02) 0.0 0.0) false false))
    (Variables|Default|SetIsActive true)
    (Utilities|FlowControl|Delay 3.0)
    (Transformation|SetWorldLocation (Variables|Default|GetRuneMesh) (Variables|Default|GetInitialLocation) false false)
    (Variables|Default|SetIsActive false)))

(event EventBeginPlay
  (Variables|Default|SetInitialLocation (Transformation|GetWorldLocation (Variables|Default|GetRuneMesh))))

(fn ConstructionScript)