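; BP_Enemy is an AI enemy that detects the player and performs a zombie melee attack.
; PawnSensing sets the SeePlayer Blackboard key on seeing a Player-tagged pawn, while a looping timer regularly clears it.
; AttackPlayer, guarded by IsAttacking, plays the attack montage and immediately sphere-traces forward from AttackTracePoint to damage the pawn it hits.
; The guard resets when the montage completes.
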(event OnSeePawn(PawnSensing)
  (params (Pawn :type Pawn%20Object%20Reference))
  ;[0.15 0.15 0.15 0.5] See Player
  (if (Actor|ActorHasTag Pawn "Player")
    (AI|Components|Blackboard|SetValueasBool (AI|GetBlackboard (AI|GetAIController self)) (Utilities|Name|MakeLiteralName "SeePlayer") true)))

(event Custom|AttackPlayer
  (bind _attack_trace_point (Variables|Default|GetAttack%20trace%20point))
  (bind _returnvalue (Transformation|GetWorldLocation _attack_trace_point))
  ;[0.15 0.15 0.15 0.5] Attack
  (if (not (Variables|Default|GetIsAttacking?))
    (Variables|Default|SetIsAttacking? true)
    (Animation|Montage|PlayMontage (Variables|Character|GetMesh) "/Game/AI/Animations/ZombieAttack_UE_Montage.ZombieAttack_UE_Montage"
      (:then
        (bind (_outhit _returnvalue_2) (Collision|SphereTraceForObjects _returnvalue (+ _returnvalue (* (Math|Vector|GetForwardVector (Transformation|GetWorldRotation _attack_trace_point)) 7e+01)) 25.0 (Utilities|Array|MakeArray "ObjectTypeQuery3") false 0 "None"))
        (if _returnvalue_2
          (Game|Damage|ApplyDamage (.HitActor (Collision|BreakHitResult _outhit)) 1e+01 0 0)))
      (:OnCompleted
        (Variables|Default|SetIsAttacking? false)))))

(event Custom|Stop%20Seeing%20Player
  ;[0.15 0.15 0.15 0.5] stop seeing player
  (AI|Components|Blackboard|SetValueasBool (AI|GetBlackboard (AI|GetAIController self)) (Utilities|Name|MakeLiteralName "SeePlayer") false))

(event EventBeginPlay
  ;[0.15 0.15 0.15 0.5] stop seeing player
  (Utilities|Time|SetTimerbyEvent (delegate Custom|Stop%20Seeing%20Player) 0.8 true))

(fn ConstructionScript)